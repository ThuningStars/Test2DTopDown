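; Player character with 2D sprites that moves on two axes, carries one item and creates the minimap widget.
; Capsule overlap auto-picks tagged items when empty-handed, and UseItem consumes a held egg to heal up to max HP.
; Dodge launches along current velocity with a brief tint and invincibility that blocks TakePhysicalDamage.
; Each tick a camera-to-player sphere trace fades blocking tilemaps, restoring them once clear; the visibility-based CameraOcclusion variant is uncalled.
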(event `self.ReceiveBeginPlay`
  (bind _returnvalue (`|CreateWidget` "/Game/Blueprints/UI/WB_Minimap.WB_Minimap_C" (`GameplayStatics.GetPlayerController` 0)))
  (`UserWidget.AddToViewport` _returnvalue 0))

(event `self.ReceiveActorBeginOverlap`
  (params (OtherActor :type "Actor Object Reference")))

(event `self.ReceiveTick`
  (params (DeltaSeconds :type "Float (single-precision)"))
  (`self.CameraOcclusionForTileMap`))

(event `InputAxis|Right`
  (params (AxisValue :type "Float (single-precision)"))
  ; Movement
  (`self.AddMovementInput` (1.0 0.0 0.0) AxisValue))

(event `InputAxis|Down`
  (params (AxisValue :type "Float (single-precision)"))
  ; Movement
  (`self.AddMovementInput` (0.0 1.0 0.0) AxisValue))

(event `self.CapsuleComponent.OnComponentBeginOverlap`
  (params (OverlappedComponent :type "PrimitiveComponent Object Reference") (OtherActor :type "Actor Object Reference") (OtherComp :type "PrimitiveComponent Object Reference") (OtherBodyIndex :type Integer) (bFromSweep :type Boolean) (SweepResult :type "HitResult Structure (by ref)"))
  ; PickUpCheck
  (if (not (`Actor.bHidden` OtherActor))
    (bind (_result _actor) (`self.IsItemInteractable` OtherActor))
    (if _result
      (bind _output_get (set `self.OverlapItem` _actor))
      (if (not (`self.IsContainItem`))
        (`self.PickUpItem` _output_get)))))

(event `self.CapsuleComponent.OnComponentEndOverlap`
  (params (OverlappedComponent :type "PrimitiveComponent Object Reference") (OtherActor :type "Actor Object Reference") (OtherComp :type "PrimitiveComponent Object Reference") (OtherBodyIndex :type Integer)))

(event `InputAction|UseItem`
  (params (Key :type "Key Structure"))
  ; UseItem
  (:`Pressed`
    (if (`self.IsContainItem`)
      (`self.UseItem`))))

(event `InputAction|Dodge`
  (params (Key :type "Key Structure"))
  (bind _sprite (`self.Sprite`))
  ; Dodge
  (:`Pressed`
    (if (not (`self.IsDodge`))
      (`self.LaunchCharacter` (* (`KismetMathLibrary.Normal` (`self.GetVelocity`)) (`self.DodgeDistance`)))
      (set `self.IsInvincible` true)
      (set `self.IsDodge` true)
      (`PaperFlipbookComponent.SetSpriteColor` _sprite (struct :`R` 1.0 :`G` 1.0 :`B` 0.598958 :`A` 1.0))
      (`KismetSystemLibrary.Delay` 0.2)
      (`PaperFlipbookComponent.SetSpriteColor` _sprite (struct :`R` 1.0 :`G` 1.0 :`B` 1.0 :`A` 1.0))
      (set `self.IsInvincible` false)
      (set `self.IsDodge` false))))

(fn `CameraOcclusion`
  (bind _walls (`self.Walls`))
  (bind (_outhit _returnvalue) (`KismetSystemLibrary.SphereTraceSingle` :`Start` (`SceneComponent.K2_GetComponentLocation` (`self.Camera`)) :`End` (+ (`SceneComponent.K2_GetComponentLocation` (`self.CapsuleComponent`)) (0.0 5.0 0.0)) :`Radius` 6.0 :`TraceChannel` "TraceTypeQuery3" :`bIgnoreSelf` false))
  (if _returnvalue
    (if (`SceneComponent.IsVisible` (`.HitComponent` (`GameplayStatics.BreakHitResult` _outhit)))
      (`KismetArrayLibrary.Array_Add` _walls (`.HitComponent` (`GameplayStatics.BreakHitResult` _outhit)))
      (for _array_element _walls
        (if (== _array_element (`.HitComponent` (`GameplayStatics.BreakHitResult` _outhit)))
          (`SceneComponent.SetVisibility` _array_element false false)
          (else
            (`SceneComponent.SetVisibility` _array_element true false)
            (`KismetArrayLibrary.Array_RemoveItem` (`self.Walls`) _array_element)))))
    (else
      (for _array_element_2 _walls
        (`SceneComponent.SetVisibility` _array_element_2 true false)
        (`KismetArrayLibrary.Array_Clear` (`self.Walls`))))))

(fn `CameraOcclusionForTileMap`
  (bind _walls (`self.Walls`))
  (bind (_outhit _returnvalue) (`KismetSystemLibrary.SphereTraceSingle` :`Start` (`SceneComponent.K2_GetComponentLocation` (`self.Camera`)) :`End` (+ (`SceneComponent.K2_GetComponentLocation` (`self.CapsuleComponent`)) (0.0 5.0 0.0)) :`Radius` 4.0 :`TraceChannel` "TraceTypeQuery3" :`bIgnoreSelf` false))
  (if _returnvalue
    (bind _aspaper_tile_map_component (cast `PaperTileMapComponent` (`.HitComponent` (`GameplayStatics.BreakHitResult` _outhit))))
    (if (== (`PaperTileMapComponent.GetTileMapColor` _aspaper_tile_map_component) (struct :`R` 1.0 :`G` 1.0 :`B` 1.0 :`A` 1.0))
      (`KismetArrayLibrary.Array_Add` _walls (`.HitComponent` (`GameplayStatics.BreakHitResult` _outhit)))
      (for _array_element _walls
        (bind _aspaper_tile_map_component_2 (cast `PaperTileMapComponent` _array_element))
        (`PaperTileMapComponent.SetTileMapColor` _aspaper_tile_map_component_2 (make `LinearColor` 1.0 1.0 1.0 0.5))))
    (else
      (for _array_element_2 _walls
        (bind _aspaper_tile_map_component_3 (cast `PaperTileMapComponent` _array_element_2))
        (`PaperTileMapComponent.SetTileMapColor` _aspaper_tile_map_component_3 (make `LinearColor` 1.0 1.0 1.0 1.0)))
      (`KismetArrayLibrary.Array_Clear` (`self.Walls`)))))

(fn `IsItemInteractable`
  (params (ItemActor :type "Actor Object Reference"))
  (returns (Result :type Boolean) (Actor :type "Actor Object Reference"))
  (return (or (`self.ActorHasTag` ItemActor (`self.PickUpItemTag`)) (`self.ActorHasTag` ItemActor (`self.InterItemTag`))) ItemActor))

(fn `PickUpItem`
  (params (Items :type "Actor Object Reference"))
  (bind _asbp_inter_item (cast `/Game/Blueprints/Pickups/BP_InterItem` Items)
    (:`then`
      (bind _result (`/Game/Blueprints/Pickups/BP_InterItem.IsItemPicked` _asbp_inter_item))
      (if (not _result)
        (`PaperSpriteComponent.SetSprite` (`self.ItemSprite`) (`/Game/Blueprints/Pickups/BP_InterItem.PickUpSprite` _asbp_inter_item))
        (`/Game/Blueprints/Pickups/BP_InterItem.UpdateItemState` _asbp_inter_item true)
        (set `self.PickedItem` (`/Game/Blueprints/Pickups/BP_InterItem.PickUpItem` _asbp_inter_item))
        (set `self.IsContainItem` true :!label _label)
        (`KismetSystemLibrary.PrintString` "PickUp")))
    (:`CastFailed`
      (bind _asbp_pick_up_item (cast `/Game/Blueprints/Pickups/BP_PickUpItem` Items))
      (`PaperSpriteComponent.SetSprite` (`self.ItemSprite`) (`PaperSpriteComponent.GetSprite` (`/Game/Blueprints/Pickups/BP_PickUpItem.PaperSprite` _asbp_pick_up_item)))
      (set `self.PickedItem` Items)
      (`self.SetActorHiddenInGame` Items true)
      (goto _label))))

(fn `TakePhysicalDamage`
  (params (Damage :type Integer))
  (if (not (`self.IsInvincible`))
    (set `self.HP` (- (`self.HP`) Damage))))

(fn `UseItem`
  (bind _hp (`self.HP`))
  (bind _totalhp (`self.TotalHP`))
  (bind _asbp_egg (cast `/Game/Blueprints/Pickups/BP_Egg` (`self.PickedItem`)))
  (switch `/Game/Blueprints/Enum/ItemType` (`/Game/Blueprints/Pickups/BP_PickUpItem.Type` _asbp_egg)
    (:`NewEnumerator0`
      (if (< _hp _totalhp)
        (bind _returnvalue (+ _hp (`/Game/Blueprints/Pickups/BP_Egg.HealNum` _asbp_egg)))
        (if (>= _returnvalue _totalhp)
          (set `self.HP` _totalhp)
          (else
            (set `self.HP` _returnvalue))))
      (`PaperSpriteComponent.SetSprite` (`self.ItemSprite`) null)
      (set `self.IsContainItem` false)
      (`self.K2_DestroyActor` (`self.PickedItem`))
      (set `self.PickedItem` null)
      (`KismetSystemLibrary.PrintString` "UseItem"))))

(fn `UserConstructionScript`)