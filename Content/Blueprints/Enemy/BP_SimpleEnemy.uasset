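; BP_SimpleEnemy is a melee enemy with a sprite that chases the player and deals contact damage.
; PlayerDetect overlaps with BP_Player toggle a flag; Tick issues AI Move To toward the player while set, pinning the sprite's tilt, and stops movement otherwise.
; Capsule overlap with BP_Player applies physical damage from MeleeATK, set in the construction script.
; MeleeAttack reports that value as a physical attack.
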(event `self.ReceiveActorBeginOverlap`
  (params (OtherActor :type "Actor Object Reference"))
  (`parent.ReceiveActorBeginOverlap` OtherActor))

(event `self.ReceiveTick`
  (params (DeltaSeconds :type "Float (single-precision)"))
  (`parent.ReceiveTick` DeltaSeconds)
  (if (`self.is`)
    (`|AIMoveTo` self (0.0 0.0 0.0) (`GameplayStatics.GetPlayerCharacter` 0)
      (:`then`
        (`SceneComponent.K2_SetWorldRotation` (`self.Sprite`) (struct :`Roll` -45.0) false false)))
    (else
      (`MovementComponent.StopMovementImmediately` (`self.CharacterMovement`)))))

(event `self.PlayerDetect.OnComponentBeginOverlap`
  (params (OverlappedComponent :type "PrimitiveComponent Object Reference") (OtherActor :type "Actor Object Reference") (OtherComp :type "PrimitiveComponent Object Reference") (OtherBodyIndex :type Integer) (bFromSweep :type Boolean) (SweepResult :type "HitResult Structure (by ref)"))
  (cast `/Game/Blueprints/Player/BP_Player` OtherActor)
  (set `self.is` true))

(event `self.PlayerDetect.OnComponentEndOverlap`
  (params (OverlappedComponent :type "PrimitiveComponent Object Reference") (OtherActor :type "Actor Object Reference") (OtherComp :type "PrimitiveComponent Object Reference") (OtherBodyIndex :type Integer))
  (cast `/Game/Blueprints/Player/BP_Player` OtherActor)
  (set `self.is` false))

(event `self.CapsuleComponent.OnComponentBeginOverlap`
  (params (OverlappedComponent :type "PrimitiveComponent Object Reference") (OtherActor :type "Actor Object Reference") (OtherComp :type "PrimitiveComponent Object Reference") (OtherBodyIndex :type Integer) (bFromSweep :type Boolean) (SweepResult :type "HitResult Structure (by ref)"))
  (bind _asbp_player (cast `/Game/Blueprints/Player/BP_Player` OtherActor))
  (`/Game/Blueprints/Player/BP_Player.TakePhysicalDamage` _asbp_player (`self.MeleeATK`)))

(fn `MeleeAttack`
  (returns (IsPhysicalAttack :type Boolean) (Damage :type Integer))
  (return true (`self.MeleeATK`)))

(fn `UserConstructionScript`
  (`parent.UserConstructionScript`)
  (set `self.MeleeATK` 5))