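; BP_InterItem is a 2D item actor that tracks whether it has been picked and shows a full or empty Paper2D sprite to match.
; UpdateItemState stores the IsPicked flag and swaps the sprite, and BeginPlay runs it to apply the initial state.
; InitialPickUpItemAndSprite casts a supplied child actor to BP_PickUpItem, then caches that item and its sprite.
; IsItemPicked exposes the flag.
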(event `self.ReceiveBeginPlay`
  (`self.UpdateItemState` (`self.IsPicked`)))

(event `self.ReceiveTick`
  (params (DeltaSeconds :type "Float (single-precision)")))

(fn `InitialPickUpItemAndSprite`
  (params (PickUpItemActor :type "ChildActorComponent Object Reference"))
  (bind _asbp_pick_up_item (cast `/Game/Blueprints/Pickups/BP_PickUpItem` (`ChildActorComponent.ChildActor` PickUpItemActor)))
  (set `self.PickUpSprite` (`PaperSpriteComponent.GetSprite` (`/Game/Blueprints/Pickups/BP_PickUpItem.PaperSprite` _asbp_pick_up_item)))
  (set `self.PickUpItem` _asbp_pick_up_item))

(fn `IsItemPicked`
  (returns (Result :type Boolean))
  (return (`self.IsPicked`)))

(fn `UpdateItemState`
  (params (IsPicked :type Boolean))
  (bind _papersprite (`self.PaperSprite`))
  (bind _output_get (set `self.IsPicked` IsPicked))
  (if _output_get
    (`PaperSpriteComponent.SetSprite` _papersprite (`self.EmptySprite`))
    (else
      (`PaperSpriteComponent.SetSprite` _papersprite (`self.FullSprite`)))))

(fn `UserConstructionScript`)